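; Shield actor Blueprint in the Defender game, with a static mesh and a health component, whose event graph is currently inactive.
; BeginPlay, OnDeath and the construction script are empty, and the overlap event is disabled.
; Disconnected leftover nodes cover collision and visibility changes, relocation, spark-effect destruction that clears the main character's CanSpawnShield, and health regeneration from that character.
; None of that leftover logic runs.
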(event OnDeath(HealthComp)
  (params (BoneName :type Name :default "None") (ShotFromDirection :type Vector :default "0, 0, 0") (HitComponent :type Primitive%20Component%20Object%20Reference) (InstigatedBy :type Controller%20Object%20Reference) (DamageCauser :type Actor%20Object%20Reference)))

(event Collision|EventActorBeginOverlap
  (params (OtherActor :type Actor%20Object%20Reference)))

(event EventBeginPlay)

(fn ConstructionScript)