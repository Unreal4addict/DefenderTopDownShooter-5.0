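; Base projectile Blueprint that resolves impacts on sphere collision, acting only when the hit has a valid physical material.
; The physical material selects particle, attached decal, sound and damage multiplier, with decal fade screen size lowered to prevent fading.
; A random roll against CriticalHitRate enlarges the particle and switches damage type for point damage.
; It then pushes physics-simulating targets, fires a radial impulse and destroys itself; PhysicMatDetermination is not called here.
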(event OnComponentHit(SphereCollision)
  (params (HitComponent :type Primitive%20Component%20Object%20Reference) (OtherActor :type Actor%20Object%20Reference) (OtherComp :type Primitive%20Component%20Object%20Reference) (NormalImpulse :type Vector :default "0, 0, 0") (Hit :type Hit%20Result%20Structure%20%28by%20ref%29))
  (Variables|Default|SetOther OtherActor)
  (Variables|Default|SetOther%20Comp OtherComp)
  (Variables|Default|SetHit Hit)
  (Variables|Default|SetPhys%20Mat (.PhysMat (Collision|BreakHitResult (Variables|Default|GetHit))))
  (Variables|Default|GetPhys%20Mat
    (:then
      (Variables|Default|SetCriticalHit (CallFunction|IsCriticalHit))
      (CallFunction|SpawnParticle)
      (bind _returnvalue (Class|GameplayStatics|SpawnDecalAttached (CallFunction|GetHitDecal (Variables|Default|GetPhys%20Mat)) "4.000000,4.000000,12.000000" (Variables|Default|GetOther%20Comp) (.HitBoneName (Collision|BreakHitResult (Variables|Default|GetHit))) (.ImpactPoint (Collision|BreakHitResult (Variables|Default|GetHit))) (Math|Rotator|MakeRotfromZ (.ImpactNormal (Collision|BreakHitResult (Variables|Default|GetHit)))) "KeepWorldPosition" 3e+01)) ; Spawn decal on surface when bullet hit
      (CallFunction|DecalSetFadeScreenSize _returnvalue) ; Prevent fading decals
      (Audio|PlaySoundatLocation (CallFunction|GetProjectileHitSound (Variables|Default|GetPhys%20Mat)) (.ImpactPoint (Collision|BreakHitResult (Variables|Default|GetHit))) "0, 0, 0" 1.0 1.0 0.0 "/Game/Defender/Demo/Audio/Attenuations/ATT_BulletImpacts.ATT_BulletImpacts" "/Game/Defender/Demo/Audio/Concurrencies/Con_BulletImpactSound.Con_BulletImpactSound" 0)
      (Variables|Default|SetHitFromDirection (Math|Vector|GetForwardVector (Transformation|GetActorRotation)))
      (if (Variables|Default|GetCriticalHit)
        (Variables|Default|SetDamage%20Type%20Class "/Game/Defender/Blueprints/DamageTypes/BP_DamageTypeCritical.BP_DamageTypeCritical_C")
        (else
          (Variables|Default|SetDamage%20Type%20Class "/Script/Engine.DamageType")))
      (Utilities|FlowControl|Sequence
        (:then_0
          (Utilities|IsValid (Components|GetOwner) ; Fix: Accessed None
            (:Is%20Valid
              (Game|Damage|ApplyPointDamage (Variables|Default|GetOther) (* (CallFunction|GetHitDamageMultiplier (Variables|Default|GetPhys%20Mat) (Variables|Attributes|GetVulnarable%20Damage%20Multiplier) (Variables|Default|GetCriticalHit)) (Variables|Attributes|GetDamage)) (Variables|Default|GetHitFromDirection) (Variables|Default|GetHit) (Game|GetInstigatorController (Components|GetOwner)) self (Variables|Default|GetDamage%20Type%20Class)) ; Apply point damage to hit actor
            )))
        (:then_1
          (CallFunction|AddImpulsetoOther)
          (Actor|DestroyActor))))
    (:else)))

(event Custom|AddImpulseToOther
  (Utilities|IsValid (Variables|Default|GetOther)
    (:Is%20Valid
      (if (Physics|IsSimulatingPhysics (Variables|/Script/Engine.Actor|GetRootComponent (Variables|Default|GetOther)) "None")
        (Physics|AddImpulse (.AsPrimitive%20Component (Utilities|Casting|CastToPrimitiveComponent (Variables|/Script/Engine.Actor|GetRootComponent (Variables|Default|GetOther)))) (* (Variables|Default|GetHitFromDirection) 2e+04) "None" false) ; Add impulse if hit actor is simulating physics
      )
      (Class|RadialForceComponent|FireImpulse (Variables|Default|GetRadialForce)) ; Fire radial impulse as well
    )))

(fn ConstructionScript)

(fn PhysicMatDetermination
  (bind _output_get (LocalVariables|SetPhysicMat (.PhysMat (Collision|BreakHitResult (Variables|Default|GetHit)))))
  (switch Utilities|FlowControl|Switch|SwitchonEPhysicalSurface (Variables|/Script/PhysicsCore.PhysicalMaterial|GetSurfaceType _output_get)
    (:SurfaceType_Default
      (LocalVariables|SetParticle "/Game/Defender/Demo/Particles/P_Impact.P_Impact")
      (LocalVariables|SetParticleScale "0.300000,0.300000,0.300000")
      (LocalVariables|SetDecalMat "/Engine/MaterialTemplates/VertexAnimation/AdvancedFlag.AdvancedFlag"))
    (:SurfaceType1
      (LocalVariables|SetParticle "/Game/Defender/Demo/Particles/P_Impact.P_Impact")
      (LocalVariables|SetParticleScale "0.500000,0.500000,0.500000"))
    (:SurfaceType2
      (LocalVariables|SetParticle "/Game/Defender/Demo/Particles/P_Impact.P_Impact")
      (LocalVariables|SetParticleScale "0.500000,0.500000,0.500000")
      (Variables|Attributes|SetDamage (* 4 (Variables|Attributes|GetDamage))))))

(fn DecalSetFadeScreenSize
  (params (Decal :type Decal%20Component%20Object%20Reference))
  (Utilities|IsValid Decal
    (:Is%20Valid
      (Rendering|Components|Decal|SetFadeScreenSize Decal 0.005) ; Prevent fading decals
    )))

(fn SpawnParticle
  (bind _hit (Variables|Default|GetHit))
  (bind _phys_mat (Variables|Default|GetPhys%20Mat))
  (bind (_particle _scale) (CallFunction|GetProjectileHitParticleEffect _phys_mat))
  (bind (_bblockinghit _binitialoverlap _time _distance _location _impactpoint _normal _impactnormal _physmat _hitactor _hitcomponent _hitbonename) (Collision|BreakHitResult _hit))
  (Variables|Default|SetHit%20Component (.HitComponent (Collision|BreakHitResult (Variables|Default|GetHit))))
  (LocalVariables|SetHitRot (Math|Rotator|MakeRotfromZ (.ImpactNormal (Collision|BreakHitResult (Variables|Default|GetHit)))))
  (LocalVariables|SetParticle _particle)
  (LocalVariables|SetScale (Math|Vector|SelectVector (* _scale 2.0) _scale (Variables|Default|GetCriticalHit)))
  (Effects|SpawnEmitterAttached (LocalVariables|GetParticle) (Variables|Default|GetHit%20Component) _hitbonename _impactpoint (LocalVariables|GetHitRot) (LocalVariables|GetScale) "KeepWorldPosition" true "AutoRelease"))

(fn IsCriticalHit
  (return (>= (Math|Float|Truncate (Math|Float|MapRangeClamped (Variables|Attributes|GetCriticalHitRate) 0.0 1.0 0.0 1e+02)) (Math|Random|RandomIntegerinRange 0 100))))