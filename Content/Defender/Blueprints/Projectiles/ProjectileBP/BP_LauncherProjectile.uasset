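; BP_LauncherProjectile is a launcher projectile that explodes when its collision sphere hits something.
; Explode spawns a pooled explosion emitter, fires a radial impulse on physics meshes, applies radial damage credited to player 0, and plays an attenuated sound before destroying the actor.
; The camera shake is centered on player 0's view target rather than the blast, so its strength ignores explosion distance for that player.
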(event OnComponentHit(SphereCollision)
  (params (HitComponent :type Primitive%20Component%20Object%20Reference) (OtherActor :type Actor%20Object%20Reference) (OtherComp :type Primitive%20Component%20Object%20Reference) (NormalImpulse :type Vector :default "0, 0, 0") (Hit :type Hit%20Result%20Structure%20%28by%20ref%29))
  (CallFunction|Explode))

(event Custom|Explode
  (Variables|Default|SetLocation (Transformation|GetWorldLocation (Variables|Character|GetMesh)))
  (Effects|SpawnEmitteratLocation "/Game/Defender/Demo/Particles/P_Explosion.P_Explosion" (Variables|Default|GetLocation) "0, 0, 0" "3.000000,3.000000,3.000000" true "AutoRelease")
  (Class|RadialForceComponent|FireImpulse (Variables|Default|GetRadialForce)) ; Fire impulse to physic simulated meshes
  (Game|Damage|ApplyRadialDamage (Variables|Default|GetDamage) (Variables|Default|GetLocation) (Variables|Default|GetEffectRadius) "/Script/Engine.DamageType" (Utilities|Array|MakeArray) self (Game|GetPlayerController 0) false "ECC_Visibility") ; Apply radial damage to all actors in range
  (Camera|PlayWorldCameraShake "/Game/Defender/Blueprints/CameraShakes/BP_ExplosionShake.BP_ExplosionShake_C" (Transformation|GetActorLocation (Pawn|GetViewTarget (Game|GetPlayerController 0))) 3e+03 5e+03) ; Shake camera a bit
  (Audio|PlaySoundatLocation "/Game/Defender/Demo/Audio/Other/SCue_Explosion.SCue_Explosion" (Transformation|GetActorLocation) "0, 0, 0" 1.0 1.0 0.0 "/Game/Defender/Demo/Audio/Attenuations/ATT_Explosions.ATT_Explosions" 0 0)
  (Actor|DestroyActor))

(fn ConstructionScript
  (|CallParentFunction))