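; Actor component that manages its owner's firearms: equipping, firing, reloading, and dropping on death.
; Equipping spawns or re-shows cached weapons from InventoryComp's slot data, attaches them to a socket and notifies listeners.
; Firing loops through a retriggerable cooldown delay, gated by health, reload, throw and hit-reaction states; reload drives AnimComp.
; Owner death detaches the equipped weapon with a physics impulse, then dissolves and destroys it.
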(event Custom|StopFiring
  (bind _equippedweapon (CallFunction|GetInvEquippedWeapon))
  (Variables|Default|SetIsFiringPressed false)
  (Variables|Default|SetIsInFiringCooldown false)
  (CallFunction|DeactiveMuzzle)
  (Utilities|IsValid _equippedweapon
    (:Is%20Valid
      (Default|DeactivateLazerSight _equippedweapon))))

(event Custom|StartFiring
  (params (TargetLocation :type Vector))
  (Variables|Default|SetTargetLocation TargetLocation)
  (Variables|Default|SetIsFiringPressed true)
  (if (CallFunction|CanStartFiring) :!label _label
    (Variables|Default|SetIsInFiringCooldown true)
    (Utilities|IsValid (CallFunction|GetInvEquippedWeapon)
      (:Is%20Valid
        (Default|Fire (CallFunction|GetInvEquippedWeapon) (Variables|Default|GetTargetLocation)) ; Fire equipped weapon
        (Utilities|FlowControl|RetriggerableDelay (CallFunction|GetEquippedWeaponCooldown)) ; Delay of equipped weapon rate of fire
        (Variables|Default|SetIsInFiringCooldown false)
        (goto _label))
      (:Is%20Not%20Valid
        (CallFunction|StopFiring)))))

(event Custom|AttemptToReload
  (Utilities|IsValid (CallFunction|GetInvEquippedWeapon)
    (:Is%20Valid
      (if (CallFunction|CanReloadEquippedWeapon)
        (Variables|Default|SetIsReloading true)
        (CallFunction|StopFiring)
        (bind _returnvalue (Audio|SpawnSoundatLocation "/Game/Defender/Demo/Audio/Weapons/AssaultRifle/SCue_AR_Reload.SCue_AR_Reload" (Transformation|GetActorLocation (Variables|Default|GetOwnerActor)) "0, 0, 0" 1.0 1.0 0.0 "/Game/Defender/Demo/Audio/Attenuations/ATT_Reload.ATT_Reload" 0))
        (Variables|Default|SetReloadSound _returnvalue)
        (Default|CallOnReloadStart)
        (Default|CallOnAnimStateChanged (Variables|Default|GetAnimComp) "NewEnumerator1")))))

(event Custom|LoadEquippedWeapon
  (params (SaveGame :type SG%20Main%20Char%20Inventory%20Object%20Reference))
  (Variables|Default|SetSG SaveGame)
  (Utilities|FlowControl|Delay 0.2)
  (Utilities|IsValid (Variables|Default|GetInventoryComp) :!label _label
    (:Is%20Valid
      (bind _equippedweapon (CallFunction|EquipWeapon (CallFunction|GetWeaponClassinUsingSlot) (Variables|Default|GetOwnerSkMesh)))
      (Utilities|IsValid _equippedweapon
        (:Is%20Valid
          (CallFunction|StopFiring))))
    (:Is%20Not%20Valid
      (Utilities|FlowControl|Delay 0.2)
      (goto _label))))

(event Custom|DroppedWeaponDissolve
  (params (Weapon :type BP%20Weapon%20Parent%20Object%20Reference))
  (Variables|Default|SetDroppedWeapon Weapon)
  (Utilities|FlowControl|Delay (Variables|Attributes|GetWeaponDissolveStartDelay))
  (Default|Execute (Variables|/Game/Defender/Blueprints/Weapons/BP_WeaponParent.BP_WeaponParent_C|GetDissolveComp (Variables|Default|GetDroppedWeapon)) (Variables|/Game/Defender/Blueprints/Weapons/BP_WeaponParent.BP_WeaponParent_C|GetMesh (Variables|Default|GetDroppedWeapon)))
  (EventDispatchers|AssignDissolveCompleted (Variables|/Game/Defender/Blueprints/Weapons/BP_WeaponParent.BP_WeaponParent_C|GetDissolveComp (Variables|Default|GetDroppedWeapon)) (delegate Custom|DissolveCompleted_Event_0)))

(event Custom|DissolveCompleted_Event_0
  (Actor|DestroyActor (Variables|Default|GetDroppedWeapon)))

(event Custom|CustomEvent_1
  (params (BoneName :type Name) (ShotFromDirection :type Vector) (HitComponent :type Primitive%20Component%20Object%20Reference) (InstigatedBy :type Controller%20Object%20Reference) (DamageCauser :type Actor%20Object%20Reference))
  (Utilities|FlowControl|Delay 0.2)
  (CallFunction|OnOwnerDeath HitComponent ShotFromDirection))

(event Custom|StopReloading
  (Variables|Default|SetIsReloading false)
  (Utilities|IsValid (Variables|Default|GetReloadSound)
    (:Is%20Valid
      (Audio|Components|Audio|Stop (Variables|Default|GetReloadSound)))))

(event EventBeginPlay
  (Utilities|FlowControl|Sequence
    (:then_0
      (Variables|Default|SetOwnerActor (Components|GetOwner)) ; Get parent actor which owned this comp
      (Utilities|IsValid (Variables|Default|GetOwnerActor)
        (:Is%20Valid
          (Variables|Default|SetOwnerSkMesh (Actor|GetComponentbyClass (Variables|Default|GetOwnerActor) "/Script/Engine.SkeletalMeshComponent"))
          (bind _output_get (Variables|Default|SetHealthComp (Actor|GetComponentbyClass (Variables|Default|GetOwnerActor) "/Game/Defender/Blueprints/Components/HealthComp.HealthComp_C")))
          (EventDispatchers|AssignOnDeath _output_get (delegate Custom|CustomEvent_1)) ; Bind event when owner death
          (Variables|Default|SetAnimComp (Actor|GetComponentbyClass (Variables|Default|GetOwnerActor) "/Game/Defender/Blueprints/Components/AnimComp.AnimComp_C")) ; Set Anim Comp for animating owner
          (Variables|Default|SetInventoryComp (Actor|GetComponentbyClass (Variables|Default|GetOwnerActor) "/Game/Defender/Blueprints/Components/InventoryComp.InventoryComp_C"))
          (Variables|Default|SetThrowComp (Actor|GetComponentbyClass (Variables|Default|GetOwnerActor) "/Game/Defender/Blueprints/Components/ThrowComp.ThrowComp_C")))))
    (:then_1
      (Variables|Default|SetWeaponClassInSlot (CallFunction|GetWeaponClassinUsingSlot))
      (CallFunction|EquipWeapon (Variables|Default|GetWeaponClassInSlot) (Variables|Default|GetOwnerSkMesh)) ; Spawn weapon and attach to weapon socket
      (Default|AddWeapontoAppropriateSlot (Variables|Default|GetInventoryComp) (Variables|Default|GetWeaponClassInSlot)) ; Add first equip weapon to appropriate \nweapon slot
    )
    (:then_2
      (if (Utilities|IsValidClass (Variables|Default|GetWeaponClassInSlot))
        (Utilities|Map|Add (Variables|/Game/Defender/Blueprints/Components/InventoryComp.InventoryComp_C|GetLootWeaponCounts (Variables|Default|GetInventoryComp)) (Utilities|GetClassDefaults (Variables|Default|GetWeaponClassInSlot)) 1) ; Add First Weapon count to LootWeaponCounts
      ))))

(fn GetGI
  (Utilities|IsValid (Variables|Default|GetGI)
    (:Is%20Valid
      _)
    (:Is%20Not%20Valid
      (bind _asbp_my_game_instance (Utilities|Casting|CastToBP_MyGameInstance (Game|GetGameInstance)))
      (Variables|Default|SetGI _asbp_my_game_instance)))
  (return (Variables|Default|GetGI)))

(fn EquipWeapon
  (params (Class :type BP%20Weapon%20Parent%20Class%20Reference) (Mesh :type Skeletal%20Mesh%20Component%20Object%20Reference))
  (bind _equippedweapon (CallFunction|GetInvEquippedWeapon))
  (LocalVariables|SetInMesh Mesh)
  (bind _output_get (LocalVariables|SetWeaponClass Class))
  (if (Utilities|IsValidClass _output_get)
    (CallFunction|HideAllWeapons)
    (LocalVariables|SetWeaponRef (.Value (Utilities|Map|Find (Variables|/Game/Defender/Blueprints/Components/InventoryComp.InventoryComp_C|GetWeaponRefs (Variables|Default|GetInventoryComp)) (LocalVariables|GetWeaponClass))))
    (Utilities|IsValid (LocalVariables|GetWeaponRef)
      (:Is%20Valid
        (Variables|/Game/Defender/Blueprints/Components/InventoryComp.InventoryComp_C|SetEquippedWeapon (Variables|Default|GetInventoryComp) (LocalVariables|GetWeaponRef))
        (Rendering|SetVisibility (Variables|/Game/Defender/Blueprints/Weapons/BP_WeaponParent.BP_WeaponParent_C|GetMesh (LocalVariables|GetWeaponRef)) true false))
      (:Is%20Not%20Valid
        (bind _returnvalue (Game|SpawnActorfromClass (LocalVariables|GetWeaponClass) (Math|Transform|MakeTransform "0, 0, 0") "AdjustIfPossibleButAlwaysSpawn" (Components|GetOwner) 0 self (Variables|Attributes|GetIsWeaponsFlashlightVisible) 0)) ; Spawn weapon
        (Variables|/Game/Defender/Blueprints/Components/InventoryComp.InventoryComp_C|SetEquippedWeapon (Variables|Default|GetInventoryComp) _returnvalue)))
    (Utilities|FlowControl|Sequence
      (:then_0
        (Utilities|Map|Add (Variables|/Game/Defender/Blueprints/Components/InventoryComp.InventoryComp_C|GetWeaponRefs (Variables|Default|GetInventoryComp)) (LocalVariables|GetWeaponClass) (CallFunction|GetInvEquippedWeapon))
        (Transformation|AttachComponentToComponent (CallFunction|GetInvEquippedWeapon) (LocalVariables|GetInMesh) (Variables|Attributes|GetWeaponSocketName) "KeepRelative" "KeepRelative" "KeepRelative" true) ; Attach the spawned weapon to weapon socket
      )
      (:then_1
        (Audio|PlaySoundatLocation "/Game/Defender/Demo/Audio/Weapons/AssaultRifle/SCue_AR_Equip.SCue_AR_Equip" (Transformation|GetActorLocation (Variables|Default|GetOwnerActor)) "0, 0, 0" 1.0 1.0 0.0 0 0 0))
      (:then_2
        (Utilities|IsValid (Getters|GetMeleeComp)
          (:Is%20Valid
            (Default|ChangeOwnertoFirearmStance (Getters|GetMeleeComp)))))
      (:then_3
        (Default|CallOnEquippedWeaponChange (LocalVariables|GetWeaponClass) (CallFunction|GetInvEquippedWeapon) (LocalVariables|GetInMesh)) ; Inform listeners\neg. Inventory
        (Default|CallOnWeaponAmmoChanged _equippedweapon (Default|GetMagazineAmmo _equippedweapon) (Default|GetInvAmmoCount _equippedweapon)) ; Call Equipped weapon Ammo Change\nEvent dispatcher
        (return (CallFunction|GetInvEquippedWeapon))))
    (else
      (Development|PrintString "Weapon class is not defined in Weapon Comp!" true true "(R=1.000000,G=0.000000,B=0.027883,A=1.000000)" 1e+02))))

(fn EquipWeaponbySlot
  (params (WeaponSlot :type WeaponSlotEnum%20Enum :default "NewEnumerator3"))
  (CallFunction|EquipWeapon (.Value (Utilities|Map|Find (Variables|/Game/Defender/Blueprints/Components/InventoryComp.InventoryComp_C|GetWeaponSlots (Variables|Default|GetInventoryComp)) WeaponSlot)) (Variables|Default|GetOwnerSkMesh)))

(fn EquipWeaponinUsingSlot
  (CallFunction|EquipWeapon (.Value (Utilities|Map|Find (Variables|/Game/Defender/Blueprints/Components/InventoryComp.InventoryComp_C|GetWeaponSlots (Variables|Default|GetInventoryComp)) (Variables|/Game/Defender/Blueprints/Components/InventoryComp.InventoryComp_C|GetUsingWeaponSlot (Variables|Default|GetInventoryComp)))) (Variables|Default|GetOwnerSkMesh)))

(fn GetWeaponClassinUsingSlot
  (return (.Value (Utilities|Map|Find (Variables|/Game/Defender/Blueprints/Components/InventoryComp.InventoryComp_C|GetWeaponSlots (Variables|Default|GetInventoryComp)) (Variables|/Game/Defender/Blueprints/Components/InventoryComp.InventoryComp_C|GetUsingWeaponSlot (Variables|Default|GetInventoryComp))))))

(fn GetWeaponReferenceinUsingSlot
  (bind _inventorycomp (Variables|Default|GetInventoryComp))
  (bind _inventorycomp_2 (Variables|Default|GetInventoryComp))
  (bind _usingweaponslot (Variables|/Game/Defender/Blueprints/Components/InventoryComp.InventoryComp_C|GetUsingWeaponSlot _inventorycomp))
  (bind _weaponslots (Variables|/Game/Defender/Blueprints/Components/InventoryComp.InventoryComp_C|GetWeaponSlots _inventorycomp_2))
  (bind (_value _returnvalue) (Utilities|Map|Find _weaponslots _usingweaponslot))
  (if _returnvalue
    (return (.Value (Utilities|Map|Find (Variables|/Game/Defender/Blueprints/Components/InventoryComp.InventoryComp_C|GetWeaponRefs (Variables|Default|GetInventoryComp)) _value)))
    (else
      (return 0))))

(fn GetEquippedWeaponCooldown
  (return (Default|GetCooldownDelay (CallFunction|GetInvEquippedWeapon))))

(fn CanReloadEquippedWeapon
  (bind _equippedweapon (CallFunction|GetInvEquippedWeapon))
  (bind _equippedweapon_2 (CallFunction|GetInvEquippedWeapon))
  (return (Math|Boolean|ANDBoolean (and (< (Default|GetMagazineAmmo _equippedweapon_2) (Variables|/Game/Defender/Blueprints/Weapons/BP_WeaponParent.BP_WeaponParent_C|GetMagazineSize _equippedweapon_2)) (!= (Default|GetInvAmmoCount _equippedweapon_2) 0)) (not (Variables|Default|GetIsReloading)) (not (Variables|/Game/Defender/Blueprints/Components/ThrowComp.ThrowComp_C|GetIsInThrowCooldown (Variables|Default|GetThrowComp))) (Math|Boolean|NANDBoolean (<= (Default|GetMagazineAmmo _equippedweapon) 0) (<= (Default|GetInvAmmoCount _equippedweapon) 0)))))

(fn CanStartFiring
  (return (Math|Boolean|ANDBoolean (Variables|Default|GetIsFiringPressed) (not (Variables|Default|GetIsReloading)) (Variables|/Game/Defender/Blueprints/Components/HealthComp.HealthComp_C|GetisAlive (Variables|Default|GetHealthComp)) (not (Variables|Default|GetIsInFiringCooldown)) (not (Variables|/Game/Defender/Blueprints/Components/ThrowComp.ThrowComp_C|GetIsInThrowCooldown (Variables|Default|GetThrowComp))) (not (Variables|Default|GetIsReactHitAnimPlaying)))))

(fn GetInvEquippedWeapon
  (return (Variables|/Game/Defender/Blueprints/Components/InventoryComp.InventoryComp_C|GetEquippedWeapon (Variables|Default|GetInventoryComp))))

(fn GetEquippedWeapon
  (return (Variables|/Game/Defender/Blueprints/Components/InventoryComp.InventoryComp_C|GetEquippedWeapon (Variables|Default|GetInventoryComp))))

(fn HideAllWeapons
  (bind _values (Utilities|Map|Values (Variables|/Game/Defender/Blueprints/Components/InventoryComp.InventoryComp_C|GetWeaponRefs (Variables|Default|GetInventoryComp))))
  (for _array_element _values
    (LocalVariables|SetWeaponRef _array_element)
    (Utilities|IsValid (LocalVariables|GetWeaponRef)
      (:Is%20Valid
        (Rendering|SetVisibility (Variables|/Game/Defender/Blueprints/Weapons/BP_WeaponParent.BP_WeaponParent_C|GetMesh (LocalVariables|GetWeaponRef)) false false)))))

(fn Reset
  (Variables|Default|SetIsFiringPressed false)
  (Variables|Default|SetIsInFiringCooldown false)
  (Variables|Default|SetIsReloading false))

(fn DeactiveMuzzle
  (bind _output_get (LocalVariables|SetEquippedWeapon (CallFunction|GetInvEquippedWeapon)))
  (Utilities|IsValid _output_get
    (:Is%20Valid
      (Components|Activation|Deactivate (Variables|/Game/Defender/Blueprints/Weapons/BP_WeaponParent.BP_WeaponParent_C|GetMuzzleParticle (LocalVariables|GetEquippedWeapon))))))

(fn OnOwnerDeath
  (params (HitComp :type Primitive%20Component%20Object%20Reference) (ShotFromDirection :type Vector))
  (Utilities|IsValid HitComp
    (:Is%20Valid
      (LocalVariables|SetInShotFromDirection ShotFromDirection)
      (LocalVariables|SetInEquippedWeapon (CallFunction|GetInvEquippedWeapon))
      (Utilities|IsValid (LocalVariables|GetInEquippedWeapon)
        (:Is%20Valid
          (LocalVariables|SetInEquippedWeaponMesh (Variables|/Game/Defender/Blueprints/Weapons/BP_WeaponParent.BP_WeaponParent_C|GetMesh (LocalVariables|GetInEquippedWeapon)))
          (Transformation|DetachFromActor (LocalVariables|GetInEquippedWeapon) "KeepWorld" "KeepWorld" "KeepWorld") ; Detach equipped weapon
          (Components|Activation|Activate (Variables|/Game/Defender/Blueprints/Weapons/BP_WeaponParent.BP_WeaponParent_C|GetRotatingMovement (LocalVariables|GetInEquippedWeapon)) false) ; Activa rotation when weapon is falling
          (Collision|SetCollisionEnabled (LocalVariables|GetInEquippedWeaponMesh) "PhysicsOnly") ; For allowing equipped weapon to falling\nthe ground
          (Physics|SetSimulatePhysics (LocalVariables|GetInEquippedWeaponMesh) true)
          (Physics|AddImpulse (LocalVariables|GetInEquippedWeaponMesh) (* (LocalVariables|GetInShotFromDirection) 5e+02) "None" false) ; Add small impulse according to \nShotFromDirection
          (Rendering|SetRenderCustomDepth (LocalVariables|GetInEquippedWeaponMesh) false) ; Remove outline
          (CallFunction|DroppedWeaponDissolve (LocalVariables|GetInEquippedWeapon)))))))

(fn GetMeleeComp
  (Utilities|IsValid (Variables|Default|GetMeleeComp)
    (:Is%20Valid
      _)
    (:Is%20Not%20Valid
      (Variables|Default|SetMeleeComp (Actor|GetComponentbyClass (Components|GetOwner) "/Game/Defender/Blueprints/Components/MeleeComp.MeleeComp_C"))))
  (return (Variables|Default|GetMeleeComp)))